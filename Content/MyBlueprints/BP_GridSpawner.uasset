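; BP_GridSpawner is an actor that spawns a centered grid of BP_Cyliner actors when play begins.
; Its construction script builds placeholder static mesh components in a MaxX by MaxY grid, spaced by Spacing and offset around the origin, and caches them in TempMeshArray.
; BeginPlay spawns a cylinder actor at each placeholder's world transform, then destroys the placeholders, so they serve as an editor-time layout preview.
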(event EventBeginPlay
  (for _array_element (Variables|Default|GetTempMeshArray)
    (Game|SpawnActorfromClass "/Game/MyBlueprints/BP_Cyliner.BP_Cyliner_C" (Transformation|GetWorldTransform _array_element) "AlwaysSpawn" "MultiplyWithRoot" 0 0))
  (for _array_element_2 (Variables|Default|GetTempMeshArray)
    (Components|DestroyComponent _array_element_2)))

(fn ConstructionScript
  (Utilities|Array|Clear (Variables|Default|GetTempMeshArray))
  (for _index (range 0 (- (Variables|Default|GetMax%20X) 1))
    (Variables|Default|SetTemp%20X _index)
    (for _index_2 (range 0 (- (Variables|Default|GetMax%20Y) 1))
      (Variables|Default|SetTemp%20Y _index_2)
      (bind _returnvalue (AddComponent|AddStaticMeshComponent false (Math|Transform|MakeTransform (- (Math|Vector|MakeVector (* (Variables|Default|GetTemp%20X) (Variables|Default|GetSpacing)) (* (Variables|Default|GetTemp%20Y) (Variables|Default|GetSpacing)) 0.0) (Math|Vector|MakeVector (/ (* (- (Variables|Default|GetMax%20X) 1) (Variables|Default|GetSpacing)) 2.0) (/ (* (- (Variables|Default|GetMax%20Y) 1) (Variables|Default|GetSpacing)) 2.0) 0.0)))))
      (Utilities|Array|Add (Variables|Default|GetTempMeshArray) _returnvalue))))