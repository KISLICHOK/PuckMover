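; BP_Cyliner is a cylinder actor whose tube, line and decal react to the offset between its base mesh and PCAnchor.
; Each tick, once that offset passes a small threshold, GetBaseAnchorVector supplies the distance and direction.
; Distance drives the tube's height, line length and decal emission through a dynamic material instance.
; Direction drives yaw, with the tube's height and rotation smoothed by FInterpTo and the line pointing opposite the offset without smoothing.
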(event EventTick
  (params (DeltaSeconds :type Float%20%28single-precision%29))
  (if (> (.Length (CallFunction|GetBaseAnchorVector false 1.0)) 2.0)
    (Variables|Default|SetDelta%20Seconds DeltaSeconds)
    (CallFunction|SetCenterTubeHeightZ (.Length (CallFunction|GetBaseAnchorVector false 1.0)))
    (CallFunction|SetCenterTubeRotZ (.RawVector (CallFunction|GetBaseAnchorVector true 1.0)))
    (CallFunction|SetDecalMatEmission (.Length (CallFunction|GetBaseAnchorVector true 1.0)))
    (CallFunction|SetLineScaleRotation)))

(event EventBeginPlay
  (bind _returnvalue (Rendering|Material|CreateDynamicMaterialInstance (Variables|Default|GetDecalRotation) :!class /Script/Engine.DecalComponent))
  (Variables|Default|SetMAT_Decal _returnvalue))

(fn ConstructionScript)

(fn GetBaseAnchorVector
  (params (Normalized? :type Boolean) (Scalar :type Float%20%28double-precision%29))
  (bind _basemesh (Variables|Default|GetBaseMesh))
  (bind _pc_anchor (Variables|Default|GetPC_Anchor))
  (bind _returnvalue (Transformation|GetWorldLocation _basemesh))
  (bind _returnvalue_2 (Transformation|GetWorldLocation _pc_anchor))
  (bind _returnvalue_3 (- _returnvalue_2 _returnvalue))
  (return (Math|Vector|VectorLength _returnvalue_3) (* (select Normalized? (Math|Vector|Normalize _returnvalue_3) _returnvalue_3) Scalar)))

(fn SetCenterTubeHeightZ
  (params (Value :type Float%20%28double-precision%29))
  (bind _output_get (Variables|Default|SetCurrentPosZ (Math|Interpolation|FInterpTo (Variables|Default|GetCurrentPosZ) (Math|Float|MapRangeClamped Value 3.0 125.0 0.0 145.0) (Variables|Default|GetDelta%20Seconds) 1e+01)))
  (Transformation|SetRelativeLocation (Variables|Default|GetTubeMesh) (Math|Vector|MakeVector 0.0 0.0 _output_get) false false))

(fn SetCenterTubeRotZ
  (params (RawVector :type Vector%20%28by%20ref%29))
  (bind _output_get (Variables|Default|SetCurrentRotZ (Math|Interpolation|FInterpTo (Variables|Default|GetCurrentRotZ) (.Yaw (Math|Rotator|BreakRotator (Math|Rotator|MakeRotfromX RawVector))) (Variables|Default|GetDelta%20Seconds) 4.0)))
  (Transformation|SetWorldRotation (Variables|Default|GetTubeMesh) (Math|Rotator|MakeRotator 0.0 0.0 _output_get) false false))

(fn SetDecalMatEmission
  (params (Value :type Float%20%28double-precision%29))
  (Rendering|Material|SetScalarParameterValue (Variables|Default|GetMAT_Decal) "Emission" (Math|Float|MapRangeClamped Value 2.0 125.0 0.0 4.0) :!class /Script/Engine.MaterialInstanceDynamic))

(fn SetLineScaleRotation
  (Transformation|SetRelativeScale3D (Variables|Default|GetLine) (Math|Vector|MakeVector (/ (.Length (CallFunction|GetBaseAnchorVector false 1.0)) 1e+01) 1.0 1.0))
  (Transformation|SetWorldRotation (Variables|Default|GetLine) (Math|Rotator|MakeRotator 0.0 0.0 (.Yaw (Math|Rotator|BreakRotator (Math|Rotator|MakeRotfromX (.RawVector (CallFunction|GetBaseAnchorVector true -1.0)))))) false false))