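; Level-control Blueprint that lets the player drag a puck mesh with the mouse under a fixed CineCamera view.
; BeginPlay switches to that camera, shows the cursor and runs fullscreen and frame-rate console commands.
; While left mouse opens a Tick gate, the puck eases toward the deprojected cursor, scaled by camera height and flattened to Z=0.
; Escape quits and P toggles pause.
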(event EventBeginPlay
  (Game|Player|SetViewTargetwithBlend (Game|GetPlayerController 0) (Variables|Default|GetCineCamera) 0.0 "VTBlend_Linear" 0.0 false)
  (Variables|/Script/Engine.PlayerController|SetbShowMouseCursor (Game|GetPlayerController 0) true)
  (Development|ExecuteConsoleCommand "fullscreen" 0)
  (Development|ExecuteConsoleCommand "t.MaxFPS60" 0))

(event EventTick
  (params (DeltaSeconds :type Float%20%28single-precision%29))
  (bind _returnvalue (Game|GetPlayerController 0))
  (bind (_worldlocation _worlddirection) (Game|Player|ConvertMouseLocationToWorldSpace _returnvalue))
  (Variables|Default|SetDelta%20Seconds DeltaSeconds)
  (Utilities|FlowControl|Gate true
    (:Exit
      (bind _output_get (Variables|Default|SetCurrentPos (Math|Interpolation|VInterpTo (Variables|Default|GetCurrentPos) (* (+ _worldlocation (* _worlddirection (.Z (Math|Vector|BreakVector (Transformation|GetActorLocation (Variables|Default|GetCineCamera)))))) "1.000000,1.000000,0.000000") (Variables|Default|GetDelta%20Seconds) 1e+01)))
      (Transformation|SetActorLocation (Variables|Default|GetPuckMesh) _output_get false false))))

(event Input|MouseEvents|LeftMouseButton
  (params (Key :type Key%20Structure :default "None"))
  (bind _returnvalue (Game|GetPlayerController 0))
  (bind (_worldlocation _worlddirection) (Game|Player|ConvertMouseLocationToWorldSpace _returnvalue))
  (:Pressed
    (Utilities|FlowControl|Gate true) ; enters at Open
  )
  (:Released
    (Utilities|FlowControl|Gate true) ; enters at Close
  ))

(event Input|KeyboardEvents|P
  (params (Key :type Key%20Structure :default "None"))
  (:Pressed
    (Utilities|FlowControl|FlipFlop
      (:A
        (Game|SetGamePaused true))
      (:B
        (Game|SetGamePaused false)))))

(event Input|KeyboardEvents|Escape
  (params (Key :type Key%20Structure :default "None"))
  (:Pressed
    (Game|QuitGame 0 "Quit" false)))

(fn ConstructionScript)